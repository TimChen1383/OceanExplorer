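; BP_InteractiveFoliage1 is an interactive foliage actor whose skeletal mesh bends under physics while being pulled toward its animated pose.
; On BeginPlay, a Physical Animation component applies motor strengths from a configurable bone downward, then those bodies simulate at half physics blend weight.
; A Control Rig component maps the complete skeletal mesh in its pre-initialize event.
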(event `self.ReceiveBeginPlay`
  (bind _physicalanimation (`self.PhysicalAnimation`))
  (bind _bonename (`self.BoneName`))
  (bind _skeletalmesh (`self.SkeletalMesh`))
  (`PhysicalAnimationComponent.SetSkeletalMeshComponent` _physicalanimation _skeletalmesh)
  (`PhysicalAnimationComponent.ApplyPhysicalAnimationSettingsBelow` _physicalanimation _bonename (make `PhysicalAnimationData` true 100.0 100.0 50.0 1.0 10.0 1.0) true)
  (`SkeletalMeshComponent.SetAllBodiesBelowSimulatePhysics` _skeletalmesh _bonename true true)
  (`SkeletalMeshComponent.SetAllBodiesBelowPhysicsBlendWeight` _skeletalmesh _bonename 0.5 false true)
  (`PhysicalAnimationComponent.SetStrengthMultiplyer` _physicalanimation 1.0))

(event `self.ControlRig.OnPreInitializeDelegate`
  (params (Component :type "ControlRigComponent Object Reference"))
  (`ControlRigComponent.AddMappedCompleteSkeletalMesh` Component (`self.SkeletalMesh`)))

(fn `UserConstructionScript`)